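; BP_EnemyBase is an enemy base Blueprint that tracks health and deals repeated contact damage to Player-tagged actors.
; Mesh overlap starts a looping one-second timer that applies BaseDamage if the overlapping actor has the tag.
; End overlap sets the timer handle to None before clearing it, so the clear misses the running timer.
; AnyDamage sets health to damage minus current health, reversing the usual subtraction, and has no death handling.
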(event `self.ReceiveBeginPlay`
  (set `self.CurrentHealth` (`self.MaxHealth`)))

(event `self.ReceiveAnyDamage`
  (params (Damage :type "Float (single-precision)") (DamageType :type "DamageType Object Reference") (InstigatedBy :type "Controller Object Reference") (DamageCauser :type "Actor Object Reference"))
  (set `self.CurrentHealth` (- Damage (`self.CurrentHealth`))))

(event `self.Mesh.OnComponentBeginOverlap`
  (params (OverlappedComponent :type "PrimitiveComponent Object Reference") (OtherActor :type "Actor Object Reference") (OtherComp :type "PrimitiveComponent Object Reference") (OtherBodyIndex :type Integer) (bFromSweep :type Boolean) (SweepResult :type "HitResult Structure (by ref)"))
  (bind _returnvalue (`KismetSystemLibrary.K2_SetTimerDelegate` (delegate `Attack`) 1.0 true))
  (set `self.AttackTimer` _returnvalue))

(event `Attack`
  (if (`self.ActorHasTag` (stale `self.Mesh.OnComponentBeginOverlap` OtherActor) "Player")
    (`GameplayStatics.ApplyDamage` (stale `self.Mesh.OnComponentBeginOverlap` OtherActor) (`self.BaseDamage`))))

(event `self.Mesh.OnComponentEndOverlap`
  (params (OverlappedComponent :type "PrimitiveComponent Object Reference") (OtherActor :type "Actor Object Reference") (OtherComp :type "PrimitiveComponent Object Reference") (OtherBodyIndex :type Integer))
  (bind _output_get (set `self.AttackTimer` (struct)))
  (`KismetSystemLibrary.K2_ClearAndInvalidateTimerHandle` _output_get))

(fn `UserConstructionScript`)