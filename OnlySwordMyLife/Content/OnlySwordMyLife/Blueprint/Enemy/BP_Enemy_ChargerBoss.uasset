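; Charger boss enemy that chases the player, attacks in close range and calls OnBossDie every tick while its health is depleted.
; Entering TraceAround starts a looping timer that turns it toward the living player and drives its velocity; the stop logic is disconnected.
; Box overlaps toggle TargetOn in the Charger AnimBP, while Hoocker overlaps apply arm damage.
; Box exit nulls the attack timer handle before clearing it, leaving the timer running.
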(event `self.ReceiveTick`
  (params (DeltaSeconds :type "Float (single-precision)"))
  (if (<= (`self.CurrentHealth`) 0.0)
    (`self.OnBossDie`)))

(event `self.Box.OnComponentBeginOverlap`
  (params (OverlappedComponent :type "PrimitiveComponent Object Reference") (OtherActor :type "Actor Object Reference") (OtherComp :type "PrimitiveComponent Object Reference") (OtherBodyIndex :type Integer) (bFromSweep :type Boolean) (SweepResult :type "HitResult Structure (by ref)"))
  (if (`self.ActorHasTag` OtherActor "Player")
    (bind _asabp_enemy_charger (cast `/Game/OnlySwordMyLife/Animation/ABP_Enemy_Charger` (`SkeletalMeshComponent.GetAnimInstance` (`self.Mesh`))))
    (set `/Game/OnlySwordMyLife/Animation/ABP_Enemy_Charger.TargetOn` true _asabp_enemy_charger)
    (`|ExecutionSequence`
      (:`then_0`
        (if (`/Game/OnlySwordMyLife/Animation/ABP_Enemy_Charger.TargetOn` _asabp_enemy_charger)
          _))
      (:`then_1`
        (bind _returnvalue (`KismetSystemLibrary.K2_SetTimerDelegate` (delegate `CorpAttack`) 2.0))
        (set `self.ChargerAttackTimer` _returnvalue)))))

(event `CorpAttack`
  (bind _asabp_enemy_charger (cast `/Game/OnlySwordMyLife/Animation/ABP_Enemy_Charger` (`SkeletalMeshComponent.GetAnimInstance` (`self.Mesh`))))
  (set `/Game/OnlySwordMyLife/Animation/ABP_Enemy_Charger.TargetOn` true _asabp_enemy_charger)
  (if (`/Game/OnlySwordMyLife/Animation/ABP_Enemy_Charger.TargetOn` _asabp_enemy_charger)
    _))

(event `self.Box.OnComponentEndOverlap`
  (params (OverlappedComponent :type "PrimitiveComponent Object Reference") (OtherActor :type "Actor Object Reference") (OtherComp :type "PrimitiveComponent Object Reference") (OtherBodyIndex :type Integer))
  (if (`self.ActorHasTag` OtherActor "Player")
    (bind _asabp_enemy_charger (cast `/Game/OnlySwordMyLife/Animation/ABP_Enemy_Charger` (`SkeletalMeshComponent.GetAnimInstance` (`self.Mesh`))))
    (set `/Game/OnlySwordMyLife/Animation/ABP_Enemy_Charger.TargetOn` false _asabp_enemy_charger)
    (bind _output_get (set `self.ChargerAttackTimer` (struct)))
    (`KismetSystemLibrary.K2_ClearAndInvalidateTimerHandle` _output_get)))

(event `self.Hoocker.OnComponentBeginOverlap`
  (params (OverlappedComponent :type "PrimitiveComponent Object Reference") (OtherActor :type "Actor Object Reference") (OtherComp :type "PrimitiveComponent Object Reference") (OtherBodyIndex :type Integer) (bFromSweep :type Boolean) (SweepResult :type "HitResult Structure (by ref)"))
  (if (`self.ActorHasTag` OtherActor "Player")
    (bind _returnvalue (`GameplayStatics.ApplyDamage` OtherActor (`self.ArmDamage`)))
    (`KismetSystemLibrary.PrintString` (`KismetStringLibrary.Conv_DoubleToString` _returnvalue))))

(event `self.TraceAround.OnComponentBeginOverlap`
  (params (OverlappedComponent :type "PrimitiveComponent Object Reference") (OtherActor :type "Actor Object Reference") (OtherComp :type "PrimitiveComponent Object Reference") (OtherBodyIndex :type Integer) (bFromSweep :type Boolean) (SweepResult :type "HitResult Structure (by ref)"))
  (if (`self.ActorHasTag` OtherActor "Player")
    (bind _returnvalue (`KismetSystemLibrary.K2_SetTimerDelegate` (delegate `TraceAndWalk`) 0.1 true))
    (set `self.TraceTimer` _returnvalue)))

(event `TraceAndWalk`
  (bind _asabp_enemy_charger (cast `/Game/OnlySwordMyLife/Animation/ABP_Enemy_Charger` (`SkeletalMeshComponent.GetAnimInstance` (`self.Mesh`))))
  (if (`/Game/OnlySwordMyLife/Animation/ABP_Enemy_Charger.TargetOn` _asabp_enemy_charger)
    (`KismetSystemLibrary.Delay` 2.0))
  (set `/Game/OnlySwordMyLife/Animation/ABP_Enemy_Charger.TraceOn` true _asabp_enemy_charger)
  (bind _asbp_main_player (cast `/Game/OnlySwordMyLife/Blueprint/BP_MainPlayer` (`GameplayStatics.GetPlayerPawn` 0)))
  (if (not (`/Game/OnlySwordMyLife/Blueprint/BP_MainPlayer.GetOnDie` _asbp_main_player))
    (`self.K2_SetActorRotation` (`KismetMathLibrary.FindLookAtRotation` (`self.K2_GetActorLocation`) (`self.K2_GetActorLocation` (`GameplayStatics.GetPlayerPawn` 0))))
    (set `MovementComponent.Velocity` (* (`self.GetActorForwardVector`) (`self.NewVar`)) (`self.CharacterMovement`))))

(event `self.TraceAround.OnComponentEndOverlap`
  (params (OverlappedComponent :type "PrimitiveComponent Object Reference") (OtherActor :type "Actor Object Reference") (OtherComp :type "PrimitiveComponent Object Reference") (OtherBodyIndex :type Integer)))

(event `DieMessege`
  (if (<= (`self.CurrentHealth`) 0.0)
    (`self.OnBossDie`)))

(fn `UserConstructionScript`
  (`parent.UserConstructionScript`))